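; BP_Player is the playable character that punches meat to build up a meat stock and spends interactions on buying upgrades.
; It sets up Enhanced Input, camera-relative movement and the player information widget.
; Montage notifies drive the punch combo, collecting from overlapped BP_Meat actors and continuing only if punch was pressed again, otherwise restoring walking.
; Interact gathers overlapped upgrade actors and buys the closest one.
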(event `self.ReceiveBeginPlay`
  (bind _returnvalue (pcsubsystem `EnhancedInputLocalPlayerSubsystem` (`GameplayStatics.GetPlayerController` 0)))
  ;[1 1 1] Begin Play
  (`/Engine/EditorBlueprintResources/StandardMacros.IsValid` _returnvalue
    (:`Is Valid`
      (`EnhancedInputSubsystemInterface.AddMappingContext` _returnvalue "/Game/Inputs/IMC_MappingContext.IMC_MappingContext" 0 (struct))
      (`self.EnableInput` null)
      (`WidgetBlueprintLibrary.SetInputMode_GameOnly` (`GameplayStatics.GetPlayerController` 0))
      (set `CharacterMovementComponent.MaxWalkSpeed` (`self.MovementSpeed`) (`self.CharacterMovement`))
      (bind _returnvalue_2 (`|CreateWidget` "/Game/Menu/Widget/WBP_PlayerInformation.WBP_PlayerInformation_C"))
      (bind _output_get (set `self.PlayerDataRef` _returnvalue_2))
      (`UserWidget.AddToViewport` _output_get 0))))

(event `EnhancedInput|/Game/Inputs/Actions/IA_MyLook`
  (params (ActionValue :type "Vector2D Structure") (ElapsedSeconds :type "Float (double-precision)") (TriggeredSeconds :type "Float (double-precision)") (InputAction :type "InputAction Object Reference" :default "/Game/Inputs/Actions/IA_MyLook.IA_MyLook"))
  ;[1 1 1] Camera
  (:`Triggered`
    (`self.AddControllerYawInput` (* ActionValue_X -1.0))
    (`self.AddControllerPitchInput` ActionValue_Y)))

(event `EnhancedInput|/Game/Inputs/Actions/IA_MyMove`
  (params (ActionValue :type "Vector2D Structure") (ElapsedSeconds :type "Float (double-precision)") (TriggeredSeconds :type "Float (double-precision)") (InputAction :type "InputAction Object Reference" :default "/Game/Inputs/Actions/IA_MyMove.IA_MyMove"))
  (bind (_returnvalue_roll _returnvalue_pitch _returnvalue_yaw) (`KismetMathLibrary.BreakRotator` (`self.GetControlRotation`)))
  ;[1 1 1] Movements
  (:`Triggered`
    (`self.AddMovementInput` (`KismetMathLibrary.GetRightVector` (`KismetMathLibrary.MakeRotator` 0.0 0.0 _returnvalue_yaw)) ActionValue_X)
    (`self.AddMovementInput` (`KismetMathLibrary.GetForwardVector` (`KismetMathLibrary.MakeRotator` 0.0 0.0 _returnvalue_yaw)) ActionValue_Y)
    (`self.K2_SetActorRotation` (`KismetMathLibrary.RInterpTo` (`self.K2_GetActorRotation`) (`KismetMathLibrary.FindLookAtRotation` (`self.K2_GetActorLocation`) (`KismetMathLibrary.MakeVector` ActionValue_X ActionValue_Y)) 0.0 5.0))))

(event `EnhancedInput|/Game/Inputs/Actions/IA_Punch`
  (params (ActionValue :type Boolean) (ElapsedSeconds :type "Float (double-precision)") (TriggeredSeconds :type "Float (double-precision)") (InputAction :type "InputAction Object Reference" :default "/Game/Inputs/Actions/IA_Punch.IA_Punch"))
  ;[1 1 1] Punch Combo
  (:`Started`
    (if (not (`self.isPunching?`))
      (set `self.isPunching?` true)
      (`CharacterMovementComponent.DisableMovement` (`self.CharacterMovement`))
      (`|PlayMontage` (`self.Mesh`) "/Game/Animations/Sequences/A_Punches_Montage.A_Punches_Montage"
        (:`OnCompleted`
          (set `self.isPunching?` false :!label _label)
          (set `self.Combo?` false :!label _label_2))
        (:`OnInterrupted`
          (goto _label))
        (:`OnNotifyBegin`
          (`self.BeatMeat`)
          (if (and (`self.isPunching?`) (`self.Combo?`))
            (goto _label_2)
            (else
              (`AnimInstance.Montage_Stop` (`SkeletalMeshComponent.GetAnimInstance` (`self.Mesh`)) 0.0 null)
              (`CharacterMovementComponent.SetMovementMode` (`self.CharacterMovement`) "MOVE_Walking" 0)))))
      (else
        (set `self.Combo?` true)))))

(event `BeatMeat`
  ;[1 1 1] Beat Meat
  (for _array_element (`PrimitiveComponent.GetOverlappingActors` (`self.Attack range`) null)
    (cast `/Game/Blueprints/BP_Meat` _array_element)
    (set `self.MeatStock` (+ (`self.MeatStock`) (`self.CurrentMeatCollect`)))
    (`/Game/Menu/Widget/WBP_PlayerInformation.UpdateScore` (`self.PlayerDataRef`))))

(event `EnhancedInput|/Game/Inputs/Actions/IA_Interact`
  (params (ActionValue :type Boolean) (ElapsedSeconds :type "Float (double-precision)") (TriggeredSeconds :type "Float (double-precision)") (InputAction :type "InputAction Object Reference" :default "/Game/Inputs/Actions/IA_Interact.IA_Interact"))
  ;[1 1 1] Check upgrade to buy
  (:`Triggered`
    (bind _outactors (`GameplayStatics.GetAllActorsOfClass` "/Game/Blueprints/Upgrades.Upgrades_C"))
    (`self.CheckForOverlappingUpgrade` _outactors)))

(fn `CheckForOverlappingUpgrade`
  (params (OverlappedUpgrades :type "Array of /Game/Blueprints/Upgrades Object Reference"))
  (locals (AllOverlappedUpgrade :type "Array of /Game/Blueprints/Upgrades Object Reference"))
  ;[1 1 1] Check overlapped upgrade
  (set `local.AllOverlappedUpgrade` (`|MakeArray`))
  (for _array_element OverlappedUpgrades
    (bind _playerinbox (`/Game/Blueprints/Upgrades.IsOverlapped` _array_element))
    (if _playerinbox
      (`KismetArrayLibrary.Array_Add` (`local.AllOverlappedUpgrade`) _array_element)))
  ;[1 1 1] Buy upgrade for closest
  (bind _closestupgrade (`/Game/Blueprints/Upgrades.CheckClosestUpgrade` _array_element (`local.AllOverlappedUpgrade`) self))
  (`/Engine/EditorBlueprintResources/StandardMacros.IsValid` _closestupgrade
    (:`Is Valid`
      (`/Game/Blueprints/Upgrades.BuyUpgrade` _closestupgrade))))

(fn `UserConstructionScript`)