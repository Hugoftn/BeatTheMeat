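; BP_Stove is an interactable cooking station that turns the player's bought flour, salt and water into a meat production upgrade.
; Overlap sets a proximity flag and shows or hides the recipe and bonus through the player's PlayerDataRef.
; On IA_Interact while near, it raises per-click and per-second meat, refreshes both displays, clears the three ingredient flags and unhides the player's Baguette actor.
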(event `self.ReceiveBeginPlay`
  (bind _asbp_player (cast `/Game/Blueprints/BP_Player` (`GameplayStatics.GetPlayerCharacter` 0)))
  (set `self.As BP Player` _asbp_player)
  (`self.EnableInput` (`GameplayStatics.GetPlayerController` 0)))

(event `EnhancedInput|/Game/Inputs/Actions/IA_Interact`
  (params (ActionValue :type Boolean) (ElapsedSeconds :type "Float (double-precision)") (TriggeredSeconds :type "Float (double-precision)") (InputAction :type "InputAction Object Reference" :default "/Game/Inputs/Actions/IA_Interact.IA_Interact"))
  (bind _as_bp_player (`self.As BP Player`))
  (bind _as_bp_player_2 (`self.As BP Player`))
  (bind _as_bp_player_3 (`self.As BP Player`))
  (bind _playerdataref (`/Game/Blueprints/BP_Player.PlayerDataRef` _as_bp_player_2))
  (:`Triggered`
    (if (`self.PlayerNear?`)
      (if (`/Game/Blueprints/BP_Player.SaltBuy?` _as_bp_player_3)
        (if (`/Game/Blueprints/BP_Player.WaterBuy?` _as_bp_player_3)
          (if (`/Game/Blueprints/BP_Player.FlourBuy?` _as_bp_player_3)
            (set `/Game/Blueprints/BP_Player.MeatBySec` (+ (`/Game/Blueprints/BP_Player.MeatBySec` _as_bp_player_2) 10) _as_bp_player_2)
            (`/Game/Menu/Widget/WBP_PlayerInformation.UpdateViandeSeconds` _playerdataref)
            (set `/Game/Blueprints/BP_Player.CurrentMeatCollect` (+ (`/Game/Blueprints/BP_Player.CurrentMeatCollect` _as_bp_player_2) 100) _as_bp_player_2)
            (`/Game/Menu/Widget/WBP_PlayerInformation.UpdateViandeClick` _playerdataref)
            (set `/Game/Blueprints/BP_Player.FlourBuy?` false _as_bp_player)
            (set `/Game/Blueprints/BP_Player.SaltBuy?` false _as_bp_player)
            (set `/Game/Blueprints/BP_Player.WaterBuy?` false _as_bp_player)
            (`self.SetActorHiddenInGame` (`/Game/Blueprints/BP_Player.Baguette` _as_bp_player) false)))))))

(event `self.ReceiveActorBeginOverlap`
  (params (OtherActor :type "Actor Object Reference"))
  ;[1 1 1] Player Near ?
  (set `self.PlayerNear?` true)
  (`/Game/Menu/Widget/WBP_PlayerInformation.Show product details` (`/Game/Blueprints/BP_Player.PlayerDataRef` (`self.As BP Player`)) "1 flour, 1 salt, 1 water " " 100 viands/coups + 10 viandes/secondes"))

(event `self.ReceiveActorEndOverlap`
  (params (OtherActor :type "Actor Object Reference"))
  ;[1 1 1] Player not near ?
  (set `self.PlayerNear?` false)
  (`/Game/Menu/Widget/WBP_PlayerInformation.Hide product details` (`/Game/Blueprints/BP_Player.PlayerDataRef` (`self.As BP Player`))))

(fn `UserConstructionScript`)