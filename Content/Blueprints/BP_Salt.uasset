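; BP_Salt is a purchasable salt pickup that the player buys with meat stock.
; Overlap events set a proximity flag and show or hide the price and bonus through the player's PlayerDataRef, without checking which actor overlapped.
; Pressing IA_Interact while the flag is set and enough meat is held deducts the cost, sets the player's SaltBuy flag and destroys the actor.
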(event `self.ReceiveBeginPlay`
  (bind _asbp_player (cast `/Game/Blueprints/BP_Player` (`GameplayStatics.GetPlayerCharacter` 0)))
  (set `self.As BP Player` _asbp_player)
  (`self.EnableInput` (`GameplayStatics.GetPlayerController` 0)))

(event `EnhancedInput|/Game/Inputs/Actions/IA_Interact`
  (params (ActionValue :type Boolean) (ElapsedSeconds :type "Float (double-precision)") (TriggeredSeconds :type "Float (double-precision)") (InputAction :type "InputAction Object Reference" :default "/Game/Inputs/Actions/IA_Interact.IA_Interact"))
  (bind _as_bp_player (`self.As BP Player`))
  (:`Triggered`
    (if (`self.PlayerNear?`)
      (if (>= (`/Game/Blueprints/BP_Player.MeatStock` (`self.As BP Player`)) 100)
        (set `/Game/Blueprints/BP_Player.SaltBuy?` true _as_bp_player)
        (set `/Game/Blueprints/BP_Player.MeatStock` (- (`/Game/Blueprints/BP_Player.MeatStock` _as_bp_player) 100) _as_bp_player)
        (`self.K2_DestroyActor`)))))

(event `self.ReceiveActorBeginOverlap`
  (params (OtherActor :type "Actor Object Reference"))
  ;[1 1 1] Player Near ?
  (set `self.PlayerNear?` true)
  (`/Game/Menu/Widget/WBP_PlayerInformation.Show product details` (`/Game/Blueprints/BP_Player.PlayerDataRef` (`self.As BP Player`)) "100" " Get salt"))

(event `self.ReceiveActorEndOverlap`
  (params (OtherActor :type "Actor Object Reference"))
  ;[1 1 1] Player not near ?
  (set `self.PlayerNear?` false)
  (`/Game/Menu/Widget/WBP_PlayerInformation.Hide product details` (`/Game/Blueprints/BP_Player.PlayerDataRef` (`self.As BP Player`))))

(fn `UserConstructionScript`)