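; Upgrade station actor that sells meat-per-second increases to BP_Player and drives that passive meat income.
; Overlap events flag proximity, and pressing A while near buys a level if MeatStock exceeds a cost that scales linearly with Level.
; A purchase raises MeatBySec and deducts the cost.
; A looping one-second timer, started on BeginPlay, adds MeatBySec to the stock, with display updates sent through the player's PlayerDataRef.
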(event `self.ReceiveBeginPlay`
  ;[1 1 1] Cast to BP_Player
  (bind _asbp_player (cast `/Game/Blueprints/BP_Player` (`GameplayStatics.GetPlayerCharacter` 0)))
  (set `self.PlayerRef` _asbp_player)
  (`self.EnableInput` (`GameplayStatics.GetPlayerController` 0))
  (`self.Timer by Sec`))

(event `Key|A`
  (params (Key :type "Key Structure"))
  ;[1 1 1] Input Action
  (:`Pressed`
    (if (`self.PlayerNear?`)
      (`self.Set Price`)
      (`self.Check Meat`)
      (if (`self.Can By`)
        (`self.Upgrade MeatBySec`)
        (`self.Set Current level`)
        (`self.Decrease Meat`)))))

(event `Set Price`
  ;[1 1 1] Upgrade the price
  (set `self.Cost` (* (+ (`self.Level`) 1) 10)))

(event `Check Meat`
  ;[1 1 1] Check If the player can by
  (if (> (`/Game/Blueprints/BP_Player.MeatStock` (`self.PlayerRef`)) (`self.Cost`))
    (set `self.Can By` true)
    (else
      (set `self.Can By` false))))

(event `self.ReceiveActorBeginOverlap`
  (params (OtherActor :type "Actor Object Reference"))
  ;[1 1 1] Player Near ?
  (set `self.PlayerNear?` true))

(event `self.ReceiveActorEndOverlap`
  (params (OtherActor :type "Actor Object Reference"))
  ;[1 1 1] Player not near ?
  (set `self.PlayerNear?` false))

(event `Upgrade MeatBySec`
  (bind _playerref (`self.PlayerRef`))
  ;[1 1 1] Upgrade Meat by sec
  (set `/Game/Blueprints/BP_Player.MeatBySec` (+ (`/Game/Blueprints/BP_Player.MeatBySec` _playerref) 1) _playerref)
  (`/Game/Menu/Widget/WBP_PlayerInformation.UpdateViandeSeconds` (`/Game/Blueprints/BP_Player.PlayerDataRef` _playerref)))

(event `Set Current level`
  ;[1 1 1] Set Current Level
  (set `self.Level` (+ (`self.Level`) 1)))

(event `Decrease Meat`
  (bind _playerref (`self.PlayerRef`))
  ;[1 1 1] Set Meat Stock
  (set `/Game/Blueprints/BP_Player.MeatStock` (- (`/Game/Blueprints/BP_Player.MeatStock` _playerref) (`self.Cost`)) _playerref)
  (`/Game/Menu/Widget/WBP_PlayerInformation.UpdateScore` (`/Game/Blueprints/BP_Player.PlayerDataRef` _playerref)))

(event `Update Meat By Sec`
  (bind _playerref (`self.PlayerRef`))
  ;[1 1 1] Update meat
  (set `/Game/Blueprints/BP_Player.MeatStock` (+ (`/Game/Blueprints/BP_Player.MeatStock` _playerref) (`/Game/Blueprints/BP_Player.MeatBySec` _playerref)) _playerref)
  (`/Game/Menu/Widget/WBP_PlayerInformation.UpdateScore` (`/Game/Blueprints/BP_Player.PlayerDataRef` _playerref)))

(event `Timer by Sec`
  ;[1 1 1] Timer all the seconds
  (`KismetSystemLibrary.K2_SetTimer` null "Update Meat By Sec" 1.0 true))

(fn `UserConstructionScript`)